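; BP_GridManager builds a square grid of GridCell actors centered on the world origin and finds the cell nearest a given position.
; On BeginPlay, PopulateGrid clears GridArray, then spawns and stores cells in nested X/Y loops using GridSize, GridWorldSize and a half-extent offset.
; GetClosestGridPosition linearly scans the stored cells by distance and returns the location of the closest one.
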(event `self.ReceiveBeginPlay`
  (`self.PopulateGrid`))

(fn `GetClosestGridPosition`
  (params (InPosition :type "Vector Structure"))
  (returns (OutPosition :type "Vector Structure"))
  (locals (ClosestPosition :type "Vector Structure") (ClosestDistance :type "Float (double-precision)") (NewLocalVar :type "Float (double-precision)"))
  (bind _output_get (set `local.ClosestPosition` (`self.K2_GetActorLocation` (`|GetArrayItem` (`self.GridArray`)))))
  (set `local.ClosestDistance` (`KismetMathLibrary.Vector_Distance` _output_get InPosition))
  (for _array_element (`self.GridArray`)
    (bind _returnvalue (`self.K2_GetActorLocation` _array_element))
    (bind _returnvalue_2 (`KismetMathLibrary.Vector_Distance` _returnvalue InPosition))
    (if (< _returnvalue_2 (`local.ClosestDistance`))
      (set `local.ClosestDistance` _returnvalue_2)
      (set `local.ClosestPosition` _returnvalue)))
  (return (`local.ClosestPosition`)))

(fn `PopulateGrid`
  (locals (WorldOffset :type "Float (double-precision)"))
  (bind _gridworldsize (`self.GridWorldSize`))
  (bind _gridworldsize_2 (`self.GridWorldSize`))
  (bind _returnvalue (`KismetMathLibrary.FTrunc` (`local.WorldOffset`)))
  (bind _returnvalue_2 (- (`self.GridSize`) 1))
  (`KismetArrayLibrary.Array_Clear` (`self.GridArray`))
  (set `local.WorldOffset` (- (* (* (`self.GridSize`) _gridworldsize) 0.5) (* _gridworldsize 0.5)))
  ;[1 1 1] Y Pos
  (for _index (range (+ _returnvalue_2 1))
    ;[1 1 1] X Pos
    (for _index_2 (range (+ _returnvalue_2 1))
      (bind _returnvalue_3 (`|SpawnActorFromClass` "/Game/GameObjects/Grid/GridCell.GridCell_C" (`KismetMathLibrary.MakeTransform` (`KismetMathLibrary.MakeVector` (`KismetMathLibrary.Conv_IntToDouble` (- (* _index_2 _gridworldsize_2) _returnvalue)) (`KismetMathLibrary.Conv_IntToDouble` (- (* _gridworldsize_2 _index) _returnvalue)))) "AlwaysSpawn" "MultiplyWithRoot" null null))
      (`KismetArrayLibrary.Array_Add` (`self.GridArray`) _returnvalue_3))))

(fn `UserConstructionScript`)