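; BP_PloppableComponent is an actor component that tracks whether its owner has a valid placement spot and shows the result visually.
; It updates on BeginPlay and listens to the owner's actor overlap events to re-evaluate.
; Placement is valid only when no actors overlap the owner.
; The state picks the valid or invalid ploppable material, applied to slot 0 of all the owner's static mesh components.
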(event `self.ReceiveBeginPlay`
  (bind _returnvalue (`self.GetOwner`))
  (add `Actor.OnActorBeginOverlap` _returnvalue (`|CreateDelegate` :!event `OnActorOverlapChanged`))
  (add `Actor.OnActorEndOverlap` _returnvalue (`|CreateDelegate` :!event `OnActorOverlapChanged`))
  (`self.UpdateState`))

(event `OnActorOverlapChanged`
  (params (OverlappedActor :type "Actor Object Reference") (OtherActor :type "Actor Object Reference"))
  (`self.UpdateState`))

(fn `UpdateState`
  (bind _returnvalue (`Actor.K2_GetComponentsByClass` (`self.GetOwner`) "/Script/Engine.StaticMeshComponent"))
  (bind _output_get (set `self.IsPlacementValid` (== (`KismetArrayLibrary.Array_Length` (`Actor.GetOverlappingActors` (`self.GetOwner`) "/Script/Engine.Actor")) 0)))
  (if _output_get
    (for _array_element _returnvalue
      (`PrimitiveComponent.SetMaterial` _array_element 0 (`self.PloppableMaterial`)))
    (else
      (for _array_element_2 _returnvalue
        (`PrimitiveComponent.SetMaterial` _array_element_2 0 (`self.InvalidPloppableMaterial`))))))