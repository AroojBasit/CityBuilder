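; BP_ClickableComponent is an actor component that makes its owner respond to mouse clicks and hovering.
; On BeginPlay it binds to the owner's click event, and to cursor-over events if a static mesh component exists.
; Clicks toggle a clicked state that swaps the mesh material between green and red, while hovering toggles custom depth rendering.
; A placement-mode flag, set through an event, suppresses all these responses.
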(event `self.ReceiveBeginPlay`
  (bind _returnvalue (`self.GetOwner`))
  (bind _returnvalue_2 (`self.GetOwner`))
  (bind _returnvalue_3 (`Actor.GetComponentByClass` _returnvalue_2 "/Script/Engine.StaticMeshComponent"))
  (add `Actor.OnClicked` _returnvalue_2 (`|CreateDelegate` :!event `OnMouseClicked`))
  (`/Engine/EditorBlueprintResources/StandardMacros.IsValid` _returnvalue_3
    (:`Is Valid`
      (set `self.StaticMeshComponent` _returnvalue_3)
      (add `Actor.OnBeginCursorOver` _returnvalue (`|CreateDelegate` :!event `OnMouseHover`))
      (add `Actor.OnEndCursorOver` _returnvalue (`|CreateDelegate` :!event `OnMouseEndHover`)))))

(event `OnMouseClicked`
  (params (TouchedActor :type "Actor Object Reference") (ButtonPressed :type "Key Structure" :default "None"))
  (if (not (`self.InPlacementMode?`))
    (set `self.IsClicked` (not (`self.IsClicked`)))
    (bind _staticmeshcomponent (`self.StaticMeshComponent`)
      (:`then`
        (if (`self.IsClicked`)
          (`PrimitiveComponent.SetMaterial` _staticmeshcomponent 0 "/Game/Materials/MI_Green.MI_Green")
          (else
            (`PrimitiveComponent.SetMaterial` _staticmeshcomponent 0 "/Game/Materials/MI_Red.MI_Red"))))
      (:`else`))))

(event `OnMouseHover`
  (params (TouchedActor :type "Actor Object Reference"))
  (if (not (`self.InPlacementMode?`))
    (`PrimitiveComponent.SetRenderCustomDepth` (`self.StaticMeshComponent`) true)))

(event `OnMouseEndHover`
  (params (TouchedActor :type "Actor Object Reference"))
  (if (not (`self.InPlacementMode?`))
    (`PrimitiveComponent.SetRenderCustomDepth` (`self.StaticMeshComponent`) false)))

(event `InPlacementMode`
  (params (`InPlacementMode?` :type Boolean))
  (set `self.InPlacementMode?` `InPlacementMode?`))